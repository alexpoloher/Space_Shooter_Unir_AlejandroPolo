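; Game mode for a space shooter that sets up an orthographic camera and background music, and tracks experience, levels and player death.
; Destroyed enemies award experience and trigger a power-up roll in BP_GeneradorPowerUps at their position.
; Each level-up raises player health and, through level 6, reweights percentage tables for enemy and power-up spawns.
; Death and power-up changes go to the HUD; GetPowerUpToSpawn is an unused stub.
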(event `self.ReceiveBeginPlay`
  (bind _returnvalue (`GameplayStatics.GetPlayerController` 0))
  ; SetUp GameMode
  (bind _asbp_space_s_hud (cast `/Game/SpaceShooter/UI/BP_SpaceS_HUD` (`PlayerController.GetHUD` (`GameplayStatics.GetPlayerController` 0))))
  (set `self.m_HUD` _asbp_space_s_hud)
  (set `self.ExperienciaNextLevel` (`|GetArrayItem` (`self.ExpNecesaria`)))
  (set `self.PorcentajeSpawnEnemies` (`|MakeArray` 100 0 0 0 0 0 0 0))
  (set `self.JugadorMuerto` false)
  (bind _outactors (`GameplayStatics.GetAllActorsOfClass` "/Game/SpaceShooter/PowerUps/BP_GeneradorPowerUps.BP_GeneradorPowerUps_C"))
  (bind _asbp_generador_power_ups (cast `/Game/SpaceShooter/PowerUps/BP_GeneradorPowerUps` (`|GetArrayItem` _outactors)))
  (set `self.GeneradorPowerUp` _asbp_generador_power_ups)
  (bind _returnvalue_2 (`|SpawnActorFromClass` "/Script/Engine.CameraActor" (`KismetMathLibrary.MakeTransform` (0.0 0.0 1080.0) (struct :`Pitch` -90.0 :`Yaw` -180.0 :`Roll` 180.0)) "Undefined" "MultiplyWithRoot" null null))
  (`CameraComponent.SetProjectionMode` (`CameraActor.CameraComponent` _returnvalue_2) "Orthographic")
  (`CameraComponent.SetOrthoWidth` (`CameraActor.CameraComponent` _returnvalue_2) 2000.0)
  (`/Engine/EditorBlueprintResources/StandardMacros.IsValid` _returnvalue
    (:`Is Valid`
      (`PlayerController.SetViewTargetWithBlend` _returnvalue _returnvalue_2 0.0 "VTBlend_Linear" 0.0 false)
      (set `PlayerController.bShowMouseCursor` false (`GameplayStatics.GetPlayerController` 0))
      (bind _returnvalue_3 (`GameplayStatics.CreateSound2D` "/Game/SpaceShooter/Sounds/S_Background.S_Background" 0.5 1.0 0.0 null false false))
      (bind _output_get (set `self.BackgroundSound` _returnvalue_3))
      (`AudioComponent.Play` _output_get 0.0)
      (bind _asbp_sspace_s_character (cast `/Game/SpaceShooter/Players/BP_SSpaceS_Character` (`GameplayStatics.GetPlayerCharacter` 0)))
      (set `self.M_SpaceCharacter` _asbp_sspace_s_character))))

(event `PlayerDead`
  ; Gestiones cuando el jugador muere
  (set `self.JugadorMuerto` true)
  (`/Game/SpaceShooter/UI/BP_SpaceS_HUD.PlayerKilled` (`self.m_HUD`))
  (`AudioComponent.Stop` (`self.BackgroundSound`)))

(event `EnemyDestroyed`
  (params (PuntosExp :type Integer) (PosDestruccion :type "Vector Structure"))
  (bind _returnvalue (+ PuntosExp (`self.Progress`)))
  ; Lógica destruir enemigo y sumar puntos de experiencia
  (`/Game/SpaceShooter/PowerUps/BP_GeneradorPowerUps.EventSpawnPowerUp` (`self.GeneradorPowerUp`) PosDestruccion (`KismetMathLibrary.RandomIntegerInRange` 1 100))
  (if (>= _returnvalue (`self.ExperienciaNextLevel`))
    (set `self.Progress` (`self.ExperienciaNextLevel`))
    (if (not (== (`self.Level`) (`self.NivelMaximo`)))
      (`self.SubirNivel`))
    (else
      (set `self.Progress` _returnvalue))))

(event `GetPowerUp`
  (params (TipoPowerUp :type String))
  ; Gestión PowerUps
  (`/Game/SpaceShooter/UI/BP_SpaceS_HUD.GetPowerUp` (`self.m_HUD`) TipoPowerUp))

(event `PerderPowerUp`
  ; Gestión PowerUps
  (`/Game/SpaceShooter/UI/BP_SpaceS_HUD.PerderPowerUp` (`self.m_HUD`)))

(event `self.ReceiveTick`
  (params (DeltaSeconds :type "Float (single-precision)")))

(fn `GetPowerUpToSpawn`
  (params (RnadomInt :type Integer))
  (returns (Class :type "Actor Class Reference")))

(fn `SubirNivel`
  (bind _m_spacecharacter (`self.M_SpaceCharacter`))
  (bind _output_get (set `self.Level` (+ (`self.Level`) 1)))
  (if (== (`self.NivelMaximo`) _output_get)
    (set `self.ExperienciaNextLevel` 99999)
    (else
      (set `self.ExperienciaNextLevel` (`|GetArrayItem` (`self.ExpNecesaria`) (- _output_get 1)))))
  (set `self.Progress` 0) ; Se vuelve a tener  de exp
  (`/Engine/EditorBlueprintResources/StandardMacros.IsValid` _m_spacecharacter
    (:`Is Valid`
      (set `/Game/SpaceShooter/Players/BP_SSpaceS_Character.VidaMaxima` (+ (`/Game/SpaceShooter/Players/BP_SSpaceS_Character.VidaMaxima` _m_spacecharacter) 20) _m_spacecharacter)
      (set `/Game/SpaceShooter/Players/BP_SSpaceS_Character.VidaActual` (+ (`/Game/SpaceShooter/Players/BP_SSpaceS_Character.VidaActual` _m_spacecharacter) 20) _m_spacecharacter)
      (switch `int` _output_get
        (:`2`
          (set `self.PorcentajeSpawnEnemies` (`|MakeArray` 50 50 0 0 0 0 0 0))
          (set `/Game/SpaceShooter/PowerUps/BP_GeneradorPowerUps.PorcentajeSpawnPowerUps` (`|MakeArray` 50 50 0 0 0 0) (`self.GeneradorPowerUp`)))
        (:`3`
          (set `self.PorcentajeSpawnEnemies` (`|MakeArray` 40 30 30 0 0 0 0 0))
          (set `/Game/SpaceShooter/PowerUps/BP_GeneradorPowerUps.PorcentajeSpawnPowerUps` (`|MakeArray` 50 50 0 0 0 0) (`self.GeneradorPowerUp`)))
        (:`4`
          (set `self.PorcentajeSpawnEnemies` (`|MakeArray` 20 20 20 20 20 0 0 0))
          (set `/Game/SpaceShooter/PowerUps/BP_GeneradorPowerUps.PorcentajeSpawnPowerUps` (`|MakeArray` 20 20 30 30 0 0) (`self.GeneradorPowerUp`)))
        (:`5`
          (set `self.PorcentajeSpawnEnemies` (`|MakeArray` 10 10 15 20 20 20 0 5))
          (set `/Game/SpaceShooter/PowerUps/BP_GeneradorPowerUps.PorcentajeSpawnPowerUps` (`|MakeArray` 15 15 25 25 20 0) (`self.GeneradorPowerUp`)))
        (:`6`
          (set `self.PorcentajeSpawnEnemies` (`|MakeArray` 10 0 10 10 28 17 20 5))
          (set `/Game/SpaceShooter/PowerUps/BP_GeneradorPowerUps.PorcentajeSpawnPowerUps` (`|MakeArray` 15 15 15 15 20 20) (`self.GeneradorPowerUp`)))))))

(fn `UserConstructionScript`)