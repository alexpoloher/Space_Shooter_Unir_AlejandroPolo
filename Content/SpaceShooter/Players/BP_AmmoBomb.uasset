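; Bomb projectile for the space shooter that explodes on a timer or on overlapping another actor, ignoring Pawns and PowerUps.
; Tick accumulates time toward TimeToExplode, while a valid overlap disables actor collision; both paths call Explotar, then DesactivarAmmo after a short delay.
; Explotar stops movement and, once only, enables the blast capsule's overlaps and visibility with particles and sound.
; Hitting a LimiteVertical boundary deactivates it without exploding.
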(event `self.ReceiveBeginPlay`
  (`parent.ReceiveBeginPlay`))

(event `self.ReceiveTick`
  (params (DeltaSeconds :type "Float (single-precision)"))
  ; Explota pasados X segundos o al detectar colisión cercana
  (`parent.ReceiveTick` DeltaSeconds)
  (bind _output_get (set `self.TimeAcum` (+ DeltaSeconds (`self.TimeAcum`))))
  (if (>= _output_get (`self.TimeToExplode`))
    (`self.Explotar`)
    (`KismetSystemLibrary.Delay` 0.2)
    (`self.DesactivarAmmo`)))

(event `self.ReceiveActorBeginOverlap`
  (params (OtherActor :type "Actor Object Reference"))
  (bind _tags (`Actor.Tags` OtherActor))
  ; Gestión colisión
  (if (`KismetArrayLibrary.Array_Contains` _tags "LimiteVertical")
    (`KismetSystemLibrary.Delay` 0.2)
    (`self.DesactivarAmmo`)
    (else
      (cast `Pawn` OtherActor ; Comprobar que no somos nosotros mismos
        (:`CastFailed`
          (if (`KismetArrayLibrary.Array_Contains` _tags "PowerUp")
            _
            (elif (not (`self.DetectandoColision`))
              (set `self.DetectandoColision` true)
              (`self.SetActorEnableCollision` false)
              (`self.Explotar`)
              (`KismetSystemLibrary.Delay` 0.2)
              (`self.DesactivarAmmo`))))))))

(fn `Explotar`
  (bind _capsuladeexplosion (`self.CapsulaDeExplosion`))
  (set `self.Speed` 0.0)
  (if (not (`self.isExploding`))
    (set `self.isExploding` true)
    (set `PrimitiveComponent.bGenerateOverlapEvents` true _capsuladeexplosion)
    (`SceneComponent.SetVisibility` _capsuladeexplosion true false)
    (`GameplayStatics.SpawnEmitterAtLocation` "/Game/StarterContent/Particles/P_Explosion.P_Explosion" (`self.K2_GetActorLocation`) (struct) (2.0 2.0 2.0))
    (`GameplayStatics.PlaySound2D` "/Game/StarterContent/Audio/Explosion02.Explosion02" 1.0 1.0 0.0 null null)))

(fn `UserConstructionScript`
  (`parent.UserConstructionScript`))