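; BP_SpaceS_Ammo is a pooled projectile in the SpaceShooter game that flies forward along its facing each tick.
; Overlapping a "Limite" actor returns it after a short delay.
; Other overlaps, except pawns and "PowerUp" or "Saw" actors, stop it once with an explosion effect and sound before the same return.
; DesactivarAmmo hides it, disables tick and collision, and adds it back to the BP_Pool found at BeginPlay.
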(event `self.ReceiveBeginPlay`
  ; SetUp
  (bind _outactors (`GameplayStatics.GetAllActorsOfClass` "/Game/SpaceShooter/Players/BP_Pool.BP_Pool_C"))
  (set `self.M_Pool` (`|GetArrayItem` _outactors)))

(event `self.ReceiveActorBeginOverlap`
  (params (OtherActor :type "Actor Object Reference"))
  (bind _tags (`Actor.Tags` OtherActor))
  ; On Collision
  (if (`KismetArrayLibrary.Array_Contains` _tags "Limite")
    (`KismetSystemLibrary.Delay` 0.2)
    (`self.DesactivarAmmo`)
    (else
      (cast `Pawn` OtherActor ; Comprobar que no somos nosotros mismos
        (:`CastFailed`
          (if (or (`KismetArrayLibrary.Array_Contains` _tags "PowerUp") (`KismetArrayLibrary.Array_Contains` _tags "Saw"))
            _
            (elif (not (`self.DetectandoColision`))
              (set `self.DetectandoColision` true)
              (`self.SetActorEnableCollision` false)
              (set `self.Speed` 0.0)
              (`GameplayStatics.SpawnEmitterAtLocation` "/Game/StarterContent/Particles/P_Explosion.P_Explosion" (`self.K2_GetActorLocation`))
              (`GameplayStatics.PlaySound2D` "/Game/StarterContent/Audio/Explosion02.Explosion02" 1.0 1.0 0.0 null null)
              (`KismetSystemLibrary.Delay` 0.2)
              (`self.DesactivarAmmo`))))))))

(event `self.ReceiveTick`
  (params (DeltaSeconds :type "Float (single-precision)"))
  ; Update Movement
  (`self.K2_SetActorLocation` (+ (`self.K2_GetActorLocation`) (* (`self.GetActorForwardVector`) (* DeltaSeconds (`self.Speed`))))))

(fn `DesactivarAmmo`
  (`self.SetActorHiddenInGame` true)
  (`self.SetActorTickEnabled` false)
  (`self.SetActorEnableCollision` false)
  (set `self.Speed` 0.0)
  (`/Game/SpaceShooter/Players/BP_Pool.AddElementToArray` (`self.M_Pool`) self))

(fn `UserConstructionScript`)