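; Player ship character for the space shooter, handling Enhanced Input movement, timer-gated firing through BP_Pool, health and death.
; Unshielded hits shake the camera, reset position and start blinking immunity; death notifies BP_SS_GameMode.
; One timed power-up runs at a time (shield, multi-fire, recharge, bomb, saw), refreshed by same-type pickups and reported to the game mode.
; Power-ups swap ammo, shorten fire delay, absorb hits or attach a saw; extra life heals instantly.
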(event `self.ReceiveBeginPlay`
  ; Setup
  (bind _asplayer_controller (cast `PlayerController` (`self.GetController`)))
  (bind _returnvalue (pcsubsystem `EnhancedInputLocalPlayerSubsystem` _asplayer_controller))
  (`/Engine/EditorBlueprintResources/StandardMacros.IsValid` _returnvalue
    (:`Is Valid`
      (`EnhancedInputSubsystemInterface.AddMappingContext` _returnvalue "/Game/SpaceShooter/Input/BP_InputMapping.BP_InputMapping" 0 (struct))
      (bind _asbp_ss_game_mode (cast `/Game/BP_SS_GameMode` (`GameplayStatics.GetGameMode`)))
      (set `self.m_GameMode` _asbp_ss_game_mode)
      (set `self.PosicionInicial` (`self.K2_GetActorLocation`))
      (set `self.VidaActual` (`self.VidaMaxima`))
      (bind _outactors (`GameplayStatics.GetAllActorsOfClass` "/Game/SpaceShooter/Players/BP_Pool.BP_Pool_C"))
      (set `self.M_Pool` (`|GetArrayItem` _outactors)))))

(event `EnhancedInput|/Game/SpaceShooter/Input/BP_InputMove`
  (params (ActionValue :type "Vector2D Structure") (ElapsedSeconds :type "Float (double-precision)") (TriggeredSeconds :type "Float (double-precision)") (InputAction :type "InputAction Object Reference" :default "/Game/SpaceShooter/Input/BP_InputMove.BP_InputMove"))
  ; Pulsar moverse
  (:`Triggered`
    (`self.AddMovementInput` (`self.GetActorRightVector`) ActionValue_X)
    (`self.AddMovementInput` (`self.GetActorForwardVector`) ActionValue_Y)))

(event `EnhancedInput|/Game/SpaceShooter/Input/BP_InputFire`
  (params (ActionValue :type Boolean) (ElapsedSeconds :type "Float (double-precision)") (TriggeredSeconds :type "Float (double-precision)") (InputAction :type "InputAction Object Reference" :default "/Game/SpaceShooter/Input/BP_InputFire.BP_InputFire"))
  ; Pulsar disparar
  (:`Triggered`
    (if (`self.PlayerIsDead`)
      _
      (elif (`self.CanFire`)
        (`self.DoFire`)
        (set `self.CanFire` false)
        (`KismetSystemLibrary.K2_SetTimerDelegate` (delegate `UpdateFire`) (`self.FireDelay`))))))

(event `UpdateFire`
  ; Pulsar disparar
  (set `self.CanFire` true))

(event `DamageActor`
  (params (Damage :type Integer))
  (bind _returnvalue (- (`self.VidaActual`) Damage))
  ; Gestión de recibir daño
  (if (`self.TienePowerUp`)
    (if (`KismetStringLibrary.EqualEqual_StrStr` (`self.PowerUpActual`) "Shield")
      (`self.QuitarEscudo`)
      (else
        (`PlayerController.ClientStartCameraShake` :`self` (`GameplayStatics.GetPlayerController` 0) :`Shake` "/Game/SpaceShooter/Camera/BP_CameraShake.BP_CameraShake_C" :!label _label) ; La cámara vibra al ser golpeado
        (`GameplayStatics.PlaySound2D` "/Game/SpaceShooter/Sounds/S_Crash.S_Crash" 1.0 1.0 0.0 null null)
        (`KismetSystemLibrary.K2_SetTimer` null "ParpadeoInmunidad" 0.1 true)
        (`KismetSystemLibrary.K2_SetTimerDelegate` (delegate `TerminarInmunidad`) 1.5) ; Después de unos segundos, ya no se es inmune de nuevo
        (set `self.EsInmune` true)
        (if (< _returnvalue 0)
          (set `self.VidaActual` 0)
          (else
            (set `self.VidaActual` _returnvalue)))
        (`self.K2_SetActorLocation` (`self.PosicionInicial`))
        (if (== (`self.VidaActual`) 0)
          (set `self.PlayerIsDead` true)
          (`MovementComponent.StopMovementImmediately` (`self.CharacterMovement`))
          (`self.SetActorHiddenInGame` true)
          (`self.SetActorEnableCollision` false)
          (`KismetSystemLibrary.Delay` 0.5)
          (`/Game/BP_SS_GameMode.PlayerDead` (`self.m_GameMode`)))))
    (else
      (goto _label))))

(event `TerminarInmunidad`
  ; Gestión de recibir daño
  (`KismetSystemLibrary.K2_ClearTimer` null "ParpadeoInmunidad")
  (`SceneComponent.SetVisibility` (`self.CapsuleComponent`) true false)
  (set `self.EsInmune` false))

(event `self.ReceiveActorBeginOverlap`
  (params (OtherActor :type "Actor Object Reference"))
  ; Gestión overlap
  (if (`KismetArrayLibrary.Array_Contains` (`Actor.Tags` OtherActor) "Enemy")
    (`KismetSystemLibrary.Delay` 0.1)
    (if (`KismetStringLibrary.EqualEqual_StrStr` (`self.PowerUpActual`) "Shield")
      (`self.QuitarEscudo`))))

(event `AplicarPowerUp`
  (params (TipoPowerUp :type String))
  ; Gestionar PowerUps
  (switch `string` TipoPowerUp
    (:`VidaExtra`
      (`self.SumarVidaExtra`))
    (:`Shield`
      (`self.RecibirEscudo`))
    (:`MultiFire`
      (`self.RecibirMultiFire`))
    (:`Recharge`
      (`self.RecibirRecharge`))
    (:`Bomb`
      (`self.RecibirBomb`))
    (:`Saw`
      (`self.RecibirSaw`))))

(event `self.ReceiveTick`
  (params (DeltaSeconds :type "Float (single-precision)"))
  ; TickEvent
  (if (`self.TienePowerUp`)
    (set `self.TiempoRestantePowerUp` (- (`self.TiempoRestantePowerUp`) DeltaSeconds))))

(fn `DoFire`
  (if (== (`self.Lifes`) 0)
    _
    (elif (`self.TienePowerUp`)
      (if (`KismetStringLibrary.EqualEqual_StrStr` (`self.PowerUpActual`) "MultiFire")
        (`/Game/SpaceShooter/Players/BP_Pool.PlayerFire` (`self.M_Pool`) (`SceneComponent.K2_GetComponentToWorld` (`self.FirePoint`)) (`self.Ammo`) true (`SceneComponent.K2_GetComponentToWorld` (`self.FirePointExtra1`)) (`SceneComponent.K2_GetComponentToWorld` (`self.FirePointExtra2`)))
        (else
          (`/Game/SpaceShooter/Players/BP_Pool.PlayerFire` :`self` (`self.M_Pool`) :`Transform` (`SceneComponent.K2_GetComponentToWorld` (`self.FirePoint`)) :`Class` (`self.Ammo`) :!label _label) ; Si no tiene power up, o el power up es otro distinto a MultiFire, dispara normal
        ))
      (else
        (goto _label)))))

(fn `ParpadeoInmunidad`
  (bind _capsulecomponent (`self.CapsuleComponent`))
  (`SceneComponent.SetVisibility` _capsulecomponent (not (`SceneComponent.bVisible` _capsulecomponent)) true)
  (if (not (and (`self.TienePowerUp`) (`KismetStringLibrary.EqualEqual_StrStr` (`self.PowerUpActual`) "Shield")))
    (`SceneComponent.SetVisibility` (`self.Shield`) false false)))

(fn `QuitarBomb`
  (set `self.Ammo` "/Game/SpaceShooter/Players/BP_SpaceS_Ammo.BP_SpaceS_Ammo_C")
  (set `self.TienePowerUp` false)
  (`/Game/BP_SS_GameMode.PerderPowerUp` (`self.m_GameMode`))
  (set `self.PowerUpActual` ""))

(fn `QuitarEscudo`
  (if (and (`self.TienePowerUp`) (`KismetStringLibrary.EqualEqual_StrStr` (`self.PowerUpActual`) "Shield"))
    (`SceneComponent.SetVisibility` (`self.Shield`) false false)
    (set `self.EsInmune` false)
    (set `self.TienePowerUp` false)
    (`GameplayStatics.PlaySound2D` "/Game/SpaceShooter/Sounds/S_PowerOff.S_PowerOff" 1.0 1.0 0.0 null null)
    (`/Game/BP_SS_GameMode.PerderPowerUp` (`self.m_GameMode`))
    (set `self.PowerUpActual` "")))

(fn `QuitarMultiFire`
  (set `self.Ammo` "/Game/SpaceShooter/Players/BP_SpaceS_Ammo.BP_SpaceS_Ammo_C")
  (set `self.TienePowerUp` false)
  (`/Game/BP_SS_GameMode.PerderPowerUp` (`self.m_GameMode`))
  (set `self.PowerUpActual` ""))

(fn `QuitarRecharge`
  (set `self.Ammo` "/Game/SpaceShooter/Players/BP_SpaceS_Ammo.BP_SpaceS_Ammo_C")
  (set `self.FireDelay` 0.5)
  (set `self.TienePowerUp` false)
  (`/Game/BP_SS_GameMode.PerderPowerUp` (`self.m_GameMode`))
  (set `self.PowerUpActual` ""))

(fn `QuitarSaw`
  (bind _spawnedsaw (`self.SpawnedSaw`))
  (`/Engine/EditorBlueprintResources/StandardMacros.IsValid` _spawnedsaw
    (:`Is Valid`
      (`self.K2_DetachFromActor` _spawnedsaw "KeepRelative" "KeepRelative" "KeepRelative")
      (`self.K2_DestroyActor` _spawnedsaw)
      (`SceneComponent.SetVisibility` (`self.CentroSaw`) false true)
      (set `self.TienePowerUp` false)
      (`/Game/BP_SS_GameMode.PerderPowerUp` (`self.m_GameMode`))
      (set `self.PowerUpActual` ""))))

(fn `RecibirBomb`
  (if (`self.TienePowerUp`)
    (if (`KismetStringLibrary.EqualEqual_StrStr` (`self.PowerUpActual`) "Bomb")
      (`KismetSystemLibrary.K2_ClearTimer` null "QuitarBomb")
      (bind _output_get (set `self.TiempoRestantePowerUp` 15.0 :!label _label))
      (`KismetSystemLibrary.K2_SetTimer` null "QuitarBomb" _output_get)
      (set `self.TienePowerUp` true)
      (`/Game/BP_SS_GameMode.GetPowerUp` (`self.m_GameMode`) "Bomb")
      (set `self.PowerUpActual` "Bomb"))
    (else
      (set `self.Ammo` "/Game/SpaceShooter/Players/BP_AmmoBomb.BP_AmmoBomb_C")
      (goto _label))))

(fn `RecibirEscudo`
  (if (`self.TienePowerUp`)
    (if (`KismetStringLibrary.EqualEqual_StrStr` (`self.PowerUpActual`) "Shield")
      (`KismetSystemLibrary.K2_ClearTimer` null "QuitarEscudo")
      (bind _output_get (set `self.TiempoRestantePowerUp` 15.0 :!label _label))
      (`KismetSystemLibrary.K2_SetTimer` null "QuitarEscudo" _output_get)
      (set `self.TienePowerUp` true)
      (`/Game/BP_SS_GameMode.GetPowerUp` (`self.m_GameMode`) "Shield")
      (set `self.PowerUpActual` "Shield"))
    (else
      (`SceneComponent.SetVisibility` (`self.Shield`) true false)
      (set `self.EsInmune` true)
      (goto _label))))

(fn `RecibirMultiFire`
  (if (`self.TienePowerUp`)
    (if (`KismetStringLibrary.EqualEqual_StrStr` (`self.PowerUpActual`) "MultiFire")
      (`KismetSystemLibrary.K2_ClearTimer` null "QuitarMultiFire")
      (bind _output_get (set `self.TiempoRestantePowerUp` 15.0 :!label _label))
      (`KismetSystemLibrary.K2_SetTimer` null "QuitarMultiFire" _output_get)
      (set `self.TienePowerUp` true)
      (`/Game/BP_SS_GameMode.GetPowerUp` (`self.m_GameMode`) "MultiFire")
      (set `self.PowerUpActual` "MultiFire"))
    (else
      (set `self.Ammo` "/Game/SpaceShooter/Players/BP_AmmoMultiFire.BP_AmmoMultiFire_C")
      (goto _label))))

(fn `RecibirRecharge`
  (if (`self.TienePowerUp`)
    (if (`KismetStringLibrary.EqualEqual_StrStr` (`self.PowerUpActual`) "Recharge")
      (`KismetSystemLibrary.K2_ClearTimer` null "QuitarRecharge")
      (bind _output_get (set `self.TiempoRestantePowerUp` 15.0 :!label _label))
      (`KismetSystemLibrary.K2_SetTimer` null "QuitarRecharge" _output_get)
      (set `self.TienePowerUp` true)
      (`/Game/BP_SS_GameMode.GetPowerUp` (`self.m_GameMode`) "Recharge")
      (set `self.PowerUpActual` "Recharge"))
    (else
      (set `self.Ammo` "/Game/SpaceShooter/Players/BP_AmmoRecharge.BP_AmmoRecharge_C")
      (set `self.FireDelay` 0.25)
      (goto _label))))

(fn `RecibirSaw`
  (if (`self.TienePowerUp`)
    (if (`KismetStringLibrary.EqualEqual_StrStr` (`self.PowerUpActual`) "Saw")
      (`KismetSystemLibrary.K2_ClearTimer` null "QuitarSaw")
      (bind _output_get (set `self.TiempoRestantePowerUp` 15.0 :!label _label))
      (`KismetSystemLibrary.K2_SetTimer` null "QuitarSaw" _output_get)
      (set `self.TienePowerUp` true)
      (`/Game/BP_SS_GameMode.GetPowerUp` (`self.m_GameMode`) "Saw")
      (set `self.PowerUpActual` "Saw"))
    (else
      (bind _returnvalue (`|SpawnActorFromClass` "/Game/SpaceShooter/Players/BP_Saw.BP_Saw_C" (`SceneComponent.K2_GetComponentToWorld` (`self.CentroSaw`)) "Undefined" "MultiplyWithRoot" null null))
      (set `self.SpawnedSaw` _returnvalue)
      (`self.K2_AttachToComponent` _returnvalue (`self.CentroSaw`) "None" "KeepWorld" "KeepRelative" "KeepRelative" true)
      (goto _label))))

(fn `SumarVidaExtra`
  (bind _returnvalue (+ (`self.VidaActual`) 25))
  (if (< (`self.VidaActual`) (`self.VidaMaxima`))
    (if (> _returnvalue (`self.VidaMaxima`))
      (set `self.VidaActual` (`self.VidaMaxima`))
      (else
        (set `self.VidaActual` _returnvalue)))))

(fn `UserConstructionScript`)