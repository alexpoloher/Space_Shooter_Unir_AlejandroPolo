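; Space shooter enemy that sweeps sideways in a random starting direction while rotating shields around its center.
; Overlapping a "Lateral" actor reverses it, raises its speed up to a cap and adds a forward diagonal, which a one-second timer removes.
; The Move override spins the shields; player contact with one triggers an explosion, damage unless immune and the enemy-destroy call.
; "Saw" overlaps destroy the enemy, passing its experience points.
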(event `self.ReceiveBeginPlay`
  (bind _returnvalue (`self.GetActorRightVector`))
  ; Setup enemigo
  (`parent.ReceiveBeginPlay`)
  (if (== (`KismetMathLibrary.RandomInteger` 2) 0)
    (bind _output_get (set `self.MovementVector` (* _returnvalue -1)))
    (set `self.OriginalMovVector` _output_get)
    (set `self.IsRight` true)
    (else
      (bind _output_get_2 (set `self.MovementVector` _returnvalue))
      (set `self.OriginalMovVector` _output_get_2)
      (set `self.IsRight` false)))
  (set `self.VerticalMovVector` (`self.GetActorForwardVector`)))

(event `self.Capsule.OnComponentBeginOverlap`
  (params (OverlappedComponent :type "PrimitiveComponent Object Reference") (OtherActor :type "Actor Object Reference") (OtherComp :type "PrimitiveComponent Object Reference") (OtherBodyIndex :type Integer) (bFromSweep :type Boolean) (SweepResult :type "HitResult Structure (by ref)"))
  (bind _returnvalue (* (`self.MovementVector`) -1))
  ; Gestión overlaps
  (`parent.ReceiveActorBeginOverlap` OtherActor)
  (if (`KismetArrayLibrary.Array_Contains` (`Actor.Tags` OtherActor) "Lateral")
    (if (`self.isRight`)
      (set `self.isRight` false)
      (set `self.MovementVector` _returnvalue)
      (else
        (set `self.isRight` true)
        (set `self.MovementVector` _returnvalue)))
    (`self.AumentarSpeedMovimiento`)
    (set `self.MovementVector` (+ (`self.VerticalMovVector`) (`self.MovementVector`))) ; Se hace un movimiento en diagonal para ir avanzando hacia abajo
    ;; Reestablecer movimiento
    (`KismetSystemLibrary.K2_SetTimerDelegate` (delegate `RestartMovementVector`) 1.0)))

(event `RestartMovementVector`
  ; Gestión overlaps
  ;; Reestablecer movimiento
  (set `self.MovementVector` (- (`self.MovementVector`) (`self.VerticalMovVector`))))

(event `self.BoxShield2.OnComponentBeginOverlap`
  (params (OverlappedComponent :type "PrimitiveComponent Object Reference") (OtherActor :type "Actor Object Reference") (OtherComp :type "PrimitiveComponent Object Reference") (OtherBodyIndex :type Integer) (bFromSweep :type Boolean) (SweepResult :type "HitResult Structure (by ref)"))
  ; Gestión overlaps
  (`self.PlayerHitShield` OtherActor))

(event `self.BoxShield1.OnComponentBeginOverlap`
  (params (OverlappedComponent :type "PrimitiveComponent Object Reference") (OtherActor :type "Actor Object Reference") (OtherComp :type "PrimitiveComponent Object Reference") (OtherBodyIndex :type Integer) (bFromSweep :type Boolean) (SweepResult :type "HitResult Structure (by ref)"))
  ; Gestión overlaps
  (`self.PlayerHitShield` OtherActor))

(event `self.BoxShield.OnComponentBeginOverlap`
  (params (OverlappedComponent :type "PrimitiveComponent Object Reference") (OtherActor :type "Actor Object Reference") (OtherComp :type "PrimitiveComponent Object Reference") (OtherBodyIndex :type Integer) (bFromSweep :type Boolean) (SweepResult :type "HitResult Structure (by ref)"))
  ; Gestión overlaps
  (`self.PlayerHitShield` OtherActor))

(event `self.ReceiveActorBeginOverlap`
  (params (OtherActor :type "Actor Object Reference"))
  ; Gestión overlaps
  (if (`KismetArrayLibrary.Array_Contains` (`Actor.Tags` OtherActor) "Saw")
    (`self.DestruirEnemigo` (`self.PuntosExp`))))

(fn `AumentarSpeedMovimiento`
  (bind _returnvalue (+ (`self.Speed`) 25.0))
  (if (<= _returnvalue 300.0)
    (set `self.Speed` _returnvalue)))

(fn `Move`
  (params (DeltaTime :type "Float (double-precision)"))
  (bind _centro (`self.Centro`))
  (`parent.Move` DeltaTime)
  (`/Engine/EditorBlueprintResources/StandardMacros.IsValid` _centro
    (:`Is Valid`
      (`SceneComponent.K2_AddLocalRotation` _centro (`KismetMathLibrary.MakeRotator` 0.0 0.0 (* DeltaTime (`self.ShieldsRotationSpeed`))) false false))))

(fn `PlayerHitShield`
  (params (OtherActor :type "Actor Object Reference"))
  (bind _asbp_sspace_s_character (cast `/Game/SpaceShooter/Players/BP_SSpaceS_Character` OtherActor))
  (`GameplayStatics.SpawnEmitterAtLocation` "/Game/StarterContent/Particles/P_Explosion.P_Explosion" (`self.K2_GetActorLocation`))
  (`GameplayStatics.PlaySound2D` "/Game/StarterContent/Audio/Explosion01.Explosion01" 1.0 1.0 0.0 null null)
  (if (not (`/Game/SpaceShooter/Players/BP_SSpaceS_Character.EsInmune` _asbp_sspace_s_character))
    (`/Game/SpaceShooter/Players/BP_SSpaceS_Character.DamageActor` _asbp_sspace_s_character (`self.DamageToDeal`)))
  (`self.OnEnemyDestroy`))

(fn `UserConstructionScript`
  (`parent.UserConstructionScript`))