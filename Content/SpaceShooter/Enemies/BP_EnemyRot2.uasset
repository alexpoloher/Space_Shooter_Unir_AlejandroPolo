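; Space shooter enemy that descends briefly on spawn, then travels sideways while rotating, starting left or right at random.
; Its Move function spins Origen and counter-rotates Capsule1 as the actor translates, switching from the descent once Tick's timer passes a random duration.
; Overlapping a "Lateral"-tagged actor reverses direction and raises rotation speed up to a cap, with a timed cooldown before the next bounce.
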(event `self.ReceiveBeginPlay`
  (bind _returnvalue (`self.GetActorRightVector`))
  ; Setup. Al inicio, podrá iniciar su movimiento hacia la derecha o hacia la izquierda de forma aleatoria
  (`parent.ReceiveBeginPlay`)
  (if (== (`KismetMathLibrary.RandomInteger` 2) 0)
    (bind _output_get (set `self.MovementVector` _returnvalue))
    (set `self.OriginalMovVector` _output_get)
    (set `self.isRight` false)
    (else
      (bind _output_get_2 (set `self.MovementVector` (* _returnvalue -1)))
      (set `self.OriginalMovVector` _output_get_2)
      (set `self.isRight` true)))
  (set `self.VerticalMovVector` (`self.GetActorForwardVector`))
  (set `self.TiempoDescenso` (`KismetMathLibrary.Conv_IntToDouble` (`KismetMathLibrary.RandomIntegerInRange` 1 2)))
  (set `self.EstaDescendiendo` true))

(event `self.ReceiveActorBeginOverlap`
  (params (OtherActor :type "Actor Object Reference"))
  (bind _returnvalue (* (`self.MovementVector`) -1))
  ; Gestión colisiones
  (`parent.ReceiveActorBeginOverlap` OtherActor)
  (if (`KismetArrayLibrary.Array_Contains` (`Actor.Tags` OtherActor) "Lateral")
    (if (`self.DetectaLateral`)
      (set `self.DetectaLateral` false)
      (`KismetSystemLibrary.K2_SetTimerDelegate` (delegate `RestartLateral`) 4.0)
      (if (`self.isRight`)
        (set `self.isRight` false)
        (set `self.MovementVector` _returnvalue)
        (else
          (set `self.isRight` true)
          (set `self.MovementVector` _returnvalue)))
      (`self.AumentarRotationSpeed`))))

(event `RestartLateral`
  ; Gestión colisiones
  (set `self.DetectaLateral` true))

(event `self.ReceiveTick`
  (params (DeltaSeconds :type "Float (single-precision)"))
  ; Gestión del descenso
  (`parent.ReceiveTick` DeltaSeconds)
  (set `self.TiempoDescendido` (+ DeltaSeconds (`self.TiempoDescendido`)))
  (if (>= (`self.TiempoDescendido`) (`self.TiempoDescenso`))
    (set `self.EstaDescendiendo` false)))

(fn `AumentarRotationSpeed`
  (bind _returnvalue (+ (`self.RotationSpeed`) 30.0))
  (if (<= _returnvalue 180.0)
    (set `self.RotationSpeed` _returnvalue)))

(fn `InicioMovimientoVertical`
  (params (DeltaTime :type "Float (double-precision)"))
  (`self.K2_SetActorLocation` (+ (`self.K2_GetActorLocation`) (* (* DeltaTime (`self.Speed`)) (`self.VerticalMovVector`)))))

(fn `Move`
  (params (DeltaTime :type "Float (double-precision)"))
  (bind _capsule1 (`self.Capsule1`))
  (bind _returnvalue (* DeltaTime (`self.RotationSpeed`)))
  (bind _returnvalue_2 (* DeltaTime (`self.RotationSpeed`)))
  (if (`self.EstaDescendiendo`)
    ; Al inicio, se mueve de forma vertical antes de empezar a rotar
    (`self.InicioMovimientoVertical` DeltaTime)
    (else
      (if (`self.isRight`)
        (`SceneComponent.K2_AddLocalRotation` (`self.Origen`) (`KismetMathLibrary.MakeRotator` 0.0 0.0 (* _returnvalue_2 -1.0)) false false) ; Le indico que rote en Z RotationSpeed grados por segundo
        (else
          (`SceneComponent.K2_AddLocalRotation` (`self.Origen`) (`KismetMathLibrary.MakeRotator` 0.0 0.0 _returnvalue_2) false false) ; Le indico que rote en Z RotationSpeed grados por segundo
        ))
      (`self.K2_SetActorLocation` (+ (`self.K2_GetActorLocation`) (* (* DeltaTime (`self.Speed`)) (`self.MovementVector`))))
      (if (`self.isRight`)
        (`SceneComponent.K2_AddLocalRotation` _capsule1 (`KismetMathLibrary.MakeRotator` 0.0 0.0 _returnvalue) false false) ; Rotará el objeto en dirección contraria a su traslación
        (else
          (`SceneComponent.K2_AddLocalRotation` _capsule1 (`KismetMathLibrary.MakeRotator` 0.0 0.0 (* _returnvalue -1.0)) false false) ; Rotará el objeto en dirección contraria a su traslación
        )))))

(fn `UserConstructionScript`
  (`parent.UserConstructionScript`))