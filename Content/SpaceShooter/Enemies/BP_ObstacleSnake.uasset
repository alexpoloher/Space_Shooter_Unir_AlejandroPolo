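; Snake obstacle enemy for the space shooter that flies forward while five capsule sections sway sideways.
; Each tick, phase-offset sines move the sections, exposing the middle nucleus as a weak point.
; "Player"-tagged nucleus hits, saws or ship collisions destroy it through the GameMode, damaging non-immune players on collision.
; The tail touching the lower screen limit removes it without scoring.
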(event `self.ReceiveBeginPlay`
  ; Setup
  (set `self.MovementVector` (`self.GetActorForwardVector`)) ; Establecemos que su vector de movimiento sea hacia delante
  (add `self.OnObstacleDestroy` (delegate `CustomEvent`)))

(event `CustomEvent`
  ; Setup
  (`KismetSystemLibrary.Delay` 0.1)
  (`self.K2_DestroyActor`))

(event `self.ReceiveTick`
  (params (DeltaSeconds :type "Float (single-precision)"))
  ; Movimiento
  (`self.Move` DeltaSeconds))

(event `self.CapsuleNucleo.OnComponentBeginOverlap`
  (params (OverlappedComponent :type "PrimitiveComponent Object Reference") (OtherActor :type "Actor Object Reference") (OtherComp :type "PrimitiveComponent Object Reference") (OtherBodyIndex :type Integer) (bFromSweep :type Boolean) (SweepResult :type "HitResult Structure (by ref)"))
  ; Gestión del núcleo del enemigo en colisiones
  (if (`KismetArrayLibrary.Array_Contains` (`Actor.Tags` OtherActor) "Player")
    (`self.DestruirObstaculo` (`self.PuntosExp`))))

(event `self.ReceiveActorBeginOverlap`
  (params (OtherActor :type "Actor Object Reference"))
  ; Gestión colisiones
  (if (`self.SeVaADestruir`)
    _
    (elif (`KismetArrayLibrary.Array_Contains` (`Actor.Tags` OtherActor) "Saw")
      (`self.DestruirObstaculo` (`self.PuntosExp`))
      (else
        (bind _asbp_sspace_s_character (cast `/Game/SpaceShooter/Players/BP_SSpaceS_Character` OtherActor))
        (`GameplayStatics.SpawnEmitterAtLocation` "/Game/StarterContent/Particles/P_Explosion.P_Explosion" (`self.K2_GetActorLocation`))
        (`GameplayStatics.PlaySound2D` "/Game/StarterContent/Audio/Explosion01.Explosion01" 1.0 1.0 0.0 null null)
        (if (`/Game/SpaceShooter/Players/BP_SSpaceS_Character.EsInmune` _asbp_sspace_s_character)
          (`self.DestruirObstaculo` 0)
          (else
            (`/Game/SpaceShooter/Players/BP_SSpaceS_Character.DamageActor` _asbp_sspace_s_character (`self.DamageToDeal`))
            (`self.DestruirObstaculo` (`self.PuntosExp`))))
        (set `self.SeVaADestruir` true)))))

(event `self.CapsuleCola.OnComponentBeginOverlap`
  (params (OverlappedComponent :type "PrimitiveComponent Object Reference") (OtherActor :type "Actor Object Reference") (OtherComp :type "PrimitiveComponent Object Reference") (OtherBodyIndex :type Integer) (bFromSweep :type Boolean) (SweepResult :type "HitResult Structure (by ref)"))
  ; Control salida de pantalla
  (if (`KismetArrayLibrary.Array_Contains` (`Actor.Tags` OtherActor) "LimiteInferiorEnemigos")
    (`KismetSystemLibrary.Delay` 0.2)
    (`self.K2_DestroyActor`)))

(fn `CalcularMovSenoidal`
  (params (FaseActual :type "Float (double-precision)") (DeltaTimeActual :type "Float (double-precision)") (Componente :type "SceneComponent Object Reference"))
  (bind _returnvalue_location (`KismetMathLibrary.BreakTransform` (`SceneComponent.GetRelativeTransform` Componente)))
  (`SceneComponent.K2_SetRelativeLocation` Componente (+ _returnvalue_location (+ (* (* (* (`KismetMathLibrary.Sin` (+ (* (`self.Tiempo`) (`self.Frecuencia`)) FaseActual)) (`self.Amplitud`)) DeltaTimeActual) (`self.GetActorRightVector`)) (0.0 0.0 0.0))) false false))

(fn `DestruirObstaculo`
  (params (Experiencia :type Integer))
  (`self.OnObstacleDestroy`)
  (bind _asbp_ss_game_mode (cast `/Game/BP_SS_GameMode` (`GameplayStatics.GetGameMode`)))
  (`/Game/BP_SS_GameMode.EnemyDestroyed` _asbp_ss_game_mode Experiencia (`self.K2_GetActorLocation`)))

(fn `Move`
  (params (DeltaTime :type "Float (double-precision)"))
  ; Cada sección de la "Serpiente", seguirá un movimiento senoidal pero con cierta fase cada una, pero dejando al descubierto el núcleo en un momento determinado  para que se le pueda matar
  (set `self.Tiempo` (+ (`self.Tiempo`) DeltaTime)) ; Se acumula el tiempo a usar en la función seno
  (`self.CalcularMovSenoidal` (`self.Fase`) DeltaTime (`self.CapsuleCola`))
  (bind _output_get (set `self.Fase` 0.4))
  (`self.CalcularMovSenoidal` _output_get DeltaTime (`self.CapsuleIntCola`))
  (bind _output_get_2 (set `self.Fase` 0.6))
  (`self.CalcularMovSenoidal` _output_get_2 DeltaTime (`self.CapsuleNucleo`))
  (bind _output_get_3 (set `self.Fase` 0.4))
  (`self.CalcularMovSenoidal` _output_get_3 DeltaTime (`self.CapsuleIntHead`))
  (bind _output_get_4 (set `self.Fase` 0.2))
  (`self.CalcularMovSenoidal` _output_get_4 DeltaTime (`self.CapsuleHead`))
  (`self.K2_SetActorLocation` (+ (`self.K2_GetActorLocation`) (* (* DeltaTime (`self.Speed`)) (`self.MovementVector`))))
  (set `self.Fase` 0.2))

(fn `UserConstructionScript`)