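; Space shooter enemy that travels sideways along a sinusoidal path, starting randomly left or right along its right vector.
; Move advances it at Speed along that direction while adding a sine-driven velocity on its forward axis, using accumulated time, amplitude, frequency and phase.
; Overlapping a LateralHorizontal-tagged actor reverses its direction once; a later hit destroys it after a short delay.
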(event `self.ReceiveBeginPlay`
  (bind _returnvalue (`self.GetActorRightVector`))
  ; Setup
  (`parent.ReceiveBeginPlay`)
  (if (== (`KismetMathLibrary.RandomInteger` 2) 0)
    (set `self.MovementVector` (* _returnvalue -1))
    (else
      (set `self.MovementVector` _returnvalue)))
  (set `self.HaRebotado` false))

(event `self.ReceiveActorBeginOverlap`
  (params (OtherActor :type "Actor Object Reference"))
  ; Gestión colisión
  (`parent.ReceiveActorBeginOverlap` OtherActor)
  (if (`KismetArrayLibrary.Array_Contains` (`Actor.Tags` OtherActor) "LateralHorizontal")
    (if (`self.HaRebotado`)
      (`KismetSystemLibrary.Delay` 0.4)
      (`self.K2_DestroyActor`)
      (else
        (set `self.MovementVector` (* (`self.MovementVector`) -1.0))
        (set `self.HaRebotado` true)))))

(fn `Move`
  (params (DeltaTime :type "Float (double-precision)"))
  ; Mov. Sinosuidal: F(t) = Amp * sin (frec * t + fase)
  (bind _output_get (set `self.Tiempo` (+ (`self.Tiempo`) DeltaTime))) ; Se acumula el tiempo a usar en la función seno
  (`self.K2_SetActorLocation` (+ (`self.K2_GetActorLocation`) (+ (* (* (* (`KismetMathLibrary.Sin` (+ (* _output_get (`self.Frecuencia`)) (`self.Fase`))) (`self.Amplitud`)) DeltaTime) (`self.GetActorForwardVector`)) (* (* (`self.Speed`) DeltaTime) (`self.MovementVector`))))))

(fn `UserConstructionScript`
  (`parent.UserConstructionScript`))