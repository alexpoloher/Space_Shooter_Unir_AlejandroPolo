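; Pooled enemy projectile for the space shooter that flies along its forward vector on Tick and damages the player.
; Overlapping a saw or player ammo hides it, while hitting a non-immune player deals damage, stops it and plays explosion effects.
; Those hits, level limits and immune players all lead after a short delay to DesactivarAmmo, which disables the actor and returns it to BP_Pool's enemy array instead of destroying it.
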(event `self.ReceiveBeginPlay`
  ; Setup
  (bind _outactors (`GameplayStatics.GetAllActorsOfClass` "/Game/SpaceShooter/Players/BP_Pool.BP_Pool_C"))
  (set `self.M_Pool` (`|GetArrayItem` _outactors)))

(event `self.ReceiveActorBeginOverlap`
  (params (OtherActor :type "Actor Object Reference"))
  (bind _tags (`Actor.Tags` OtherActor))
  ; On Collision
  (if (`self.HaChocado`)
    _
    (elif (or (`KismetArrayLibrary.Array_Contains` _tags "Saw") (`KismetArrayLibrary.Array_Contains` _tags "AmmoJugador"))
      (`SceneComponent.SetVisibility` (`self.Capsule`) false true)
      (set `self.HaChocado` true)
      (`KismetSystemLibrary.Delay` 0.2)
      (`self.DesactivarAmmo`)
      (elif (`KismetArrayLibrary.Array_Contains` _tags "Limite")
        (`KismetSystemLibrary.Delay` 0.2 :!label _label)
        (`self.DesactivarAmmo`)
        (else
          (bind _asbp_sspace_s_character (cast `/Game/SpaceShooter/Players/BP_SSpaceS_Character` OtherActor))
          (if (`/Game/SpaceShooter/Players/BP_SSpaceS_Character.EsInmune` _asbp_sspace_s_character)
            (goto _label)
            (else
              (`/Game/SpaceShooter/Players/BP_SSpaceS_Character.DamageActor` _asbp_sspace_s_character (`self.DamageToDeal`))
              (`self.SetActorEnableCollision` false) ; Cada bala solo va a golpear una vez
              (set `self.Speed` 0.0)
              (`GameplayStatics.SpawnEmitterAtLocation` "/Game/StarterContent/Particles/P_Explosion.P_Explosion" (`self.K2_GetActorLocation`))
              (`GameplayStatics.PlaySound2D` "/Game/StarterContent/Audio/Explosion02.Explosion02" 1.0 1.0 0.0 null null)
              (`KismetSystemLibrary.Delay` 0.2)
              (`self.DesactivarAmmo`))))))))

(event `self.ReceiveTick`
  (params (DeltaSeconds :type "Float (single-precision)"))
  ; Update Movement
  (`self.K2_SetActorLocation` (+ (`self.K2_GetActorLocation`) (* (`self.GetActorForwardVector`) (* DeltaSeconds (`self.Speed`))))))

(fn `DesactivarAmmo`
  (`self.SetActorHiddenInGame` true)
  (`SceneComponent.SetVisibility` (`self.Capsule`) true true)
  (`self.SetActorTickEnabled` false)
  (`self.SetActorEnableCollision` false)
  (set `self.Speed` 0.0)
  (`/Game/SpaceShooter/Players/BP_Pool.AddElementToEnemyArray` (`self.M_Pool`) self))

(fn `UserConstructionScript`)