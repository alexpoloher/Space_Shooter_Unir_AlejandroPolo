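; Rotating space shooter enemy that travels along its initial forward vector while spinning and firing on a timer.
; Tick moves the actor, yaws its Origen component and periodically requests ammo from BP_Pool at FirePoint.
; Saw or player contact destroys it through the OnEnemyDestroy dispatcher and reports experience to the game mode, with none for ramming an immune player.
; Non-immune players take damage; the lower enemy limit removes it silently.
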(event `self.ReceiveBeginPlay`
  ; Setup enemigo
  (set `self.MovementVector` (`self.GetActorForwardVector`)) ; Establecemos que su vector de movimiento sea hacia delante
  (add `self.OnEnemyDestroy` (delegate `Destroyed_Event`))
  (bind _outactors (`GameplayStatics.GetAllActorsOfClass` "/Game/SpaceShooter/Players/BP_Pool.BP_Pool_C"))
  (set `self.M_Pool` (`|GetArrayItem` _outactors)))

(event `Destroyed_Event`
  ; Setup enemigo
  (`KismetSystemLibrary.Delay` 0.0)
  (`self.K2_DestroyActor`))

(event `self.ReceiveTick`
  (params (DeltaSeconds :type "Float (single-precision)"))
  ; Cada tick se gestiona el movimiento y si puede disparar
  (`self.Move` DeltaSeconds)
  (bind _output_get (set `self.ShootCurrentTime` (+ DeltaSeconds (`self.ShootCurrentTime`))))
  (if (> _output_get (`self.DelayShoot`))
    (set `self.ShootCurrentTime` 0.0) ; Se vuelve a poner a 0 para volver a contar cuánto tiempo desde el último disparo
    (`self.Fire`)))

(event `self.ReceiveActorBeginOverlap`
  (params (OtherActor :type "Actor Object Reference"))
  (bind _tags (`Actor.Tags` OtherActor))
  (bind _capsule1 (`self.Capsule1`))
  (if (`self.SeVaADestruir`)
    _
    (elif (`KismetArrayLibrary.Array_Contains` _tags "Saw")
      (`self.DestruirEnemigo` (`self.PuntosExp`))
      (elif (`KismetArrayLibrary.Array_Contains` _tags "LimiteInferiorEnemigos")
        (`KismetSystemLibrary.Delay` 0.2)
        (`self.K2_DestroyActor`)
        (elif (`KismetArrayLibrary.Array_Contains` _tags "Player")
          (bind _asbp_sspace_s_character (cast `/Game/SpaceShooter/Players/BP_SSpaceS_Character` OtherActor)
            (:`then`
              (`/Engine/EditorBlueprintResources/StandardMacros.IsValid` _capsule1
                (:`Is Valid`
                  (`GameplayStatics.SpawnEmitterAtLocation` "/Game/StarterContent/Particles/P_Explosion.P_Explosion" (`SceneComponent.K2_GetComponentLocation` _capsule1))
                  (`GameplayStatics.PlaySound2D` "/Game/StarterContent/Audio/Explosion01.Explosion01" 1.0 1.0 0.0 null null))
                (:`Is Not Valid`
                  _))
              (if (`/Game/SpaceShooter/Players/BP_SSpaceS_Character.EsInmune` _asbp_sspace_s_character)
                (`self.DestruirEnemigo` 0) ; Si chocas con un enemigo mientras eres inmune, no sumas experiencia a pesar de que le destruyas
                (else
                  (`/Game/SpaceShooter/Players/BP_SSpaceS_Character.DamageActor` _asbp_sspace_s_character (`self.DamageToDeal`))
                  (`self.DestruirEnemigo` (`self.PuntosExp`) :!label _label))))
            (:`CastFailed`
              (goto _label)))
          (set `self.SeVaADestruir` true))))))

(fn `DestruirEnemigo`
  (params (Experiencia :type Integer))
  (`self.OnEnemyDestroy`)
  (bind _asbp_ss_game_mode (cast `/Game/BP_SS_GameMode` (`GameplayStatics.GetGameMode`)))
  (`/Game/BP_SS_GameMode.EnemyDestroyed` _asbp_ss_game_mode Experiencia (`SceneComponent.K2_GetComponentLocation` (`self.Base`))))

(fn `Fire`
  (bind _firepoint (`self.FirePoint`))
  (`/Engine/EditorBlueprintResources/StandardMacros.IsValid` _firepoint
    (:`Is Valid`
      (`/Game/SpaceShooter/Players/BP_Pool.EnemyFire` :`self` (`self.M_Pool`) :`Class` (`self.Ammo`) :`Transform` (`SceneComponent.K2_GetComponentToWorld` _firepoint)))))

(fn `Move`
  (params (DeltaTime :type "Float (double-precision)"))
  (`SceneComponent.K2_AddLocalRotation` (`self.Origen`) (`KismetMathLibrary.MakeRotator` 0.0 0.0 (* DeltaTime (`self.RotationSpeed`))) false false) ; Le indico que rote en Z RotationSpeed grados por segundo
  (`self.K2_SetActorLocation` (+ (`self.K2_GetActorLocation`) (* (* DeltaTime (`self.Speed`)) (`self.MovementVector`)))))

(fn `UserConstructionScript`)