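; BP_EnemyH is the horizontal enemy of the space shooter, a child Blueprint that sweeps sideways and fires more often as it bounces.
; BeginPlay randomly picks right or left as the starting MovementVector, which this graph only sets.
; Overlapping an actor tagged "Lateral" reverses direction, and each right-to-left flip lowers DelayShoot one step unless it exactly equals the intended minimum, a float equality check.
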(event `self.ReceiveBeginPlay`
  (bind _returnvalue (`self.GetActorRightVector`))
  ; SetUp del enemigo horizontal
  (`parent.ReceiveBeginPlay`)
  (if (== (`KismetMathLibrary.RandomInteger` 2) 0)
    (set `self.MovementVector` _returnvalue)
    (set `self.IsRight` true)
    (else
      (set `self.MovementVector` (* _returnvalue -1))
      (set `self.IsRight` false))))

(event `self.ReceiveActorBeginOverlap`
  (params (OtherActor :type "Actor Object Reference"))
  (bind _returnvalue (`self.GetActorRightVector`))
  (bind _delayshoot (`self.DelayShoot`))
  ; Gestionar movimiento lateral (De der. a izq.)
  (`parent.ReceiveActorBeginOverlap` OtherActor)
  (if (`KismetArrayLibrary.Array_Contains` (`Actor.Tags` OtherActor) "Lateral")
    (if (`self.IsRight`)
      (set `self.IsRight` false)
      (set `self.MovementVector` (* _returnvalue -1)) ; Irá ahora hacia la izquierda
      (if (== _delayshoot 0.1)
        (set `self.DelayShoot` _delayshoot) ; Si la frecuencia de disparo y aes 0.1, no se reduce más
        (else
          (set `self.DelayShoot` (- _delayshoot 0.1)) ; Cada vez que choque para ir a la izq, aumentará su frecuencia de disparo
        ))
      (else
        (set `self.IsRight` true)
        (set `self.MovementVector` _returnvalue) ; Irá ahora hacia la derecha
      ))))

(fn `UserConstructionScript`
  (`parent.UserConstructionScript`))