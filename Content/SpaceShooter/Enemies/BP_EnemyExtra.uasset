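; BP_EnemyExtra is a space shooter enemy that crosses sideways while spinning constantly and fires from four fire points.
; It extends a parent enemy, setting MovementVector to its right vector and adding yaw rotation on Tick.
; Overlapping a "LateralHorizontal" actor reverses its direction once; the next such overlap destroys it after a short delay.
; Fire passes all four transforms to MPool.EnemyFire in one pooled call; older SpawnActor logic remains disconnected.
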(event `self.ReceiveBeginPlay`
  ; Setup
  (`parent.ReceiveBeginPlay`)
  (set `self.MovementVector` (`self.GetActorRightVector`))
  (set `self.HaRebotadoYa` false))

(event `self.ReceiveActorBeginOverlap`
  (params (OtherActor :type "Actor Object Reference"))
  ; Gestión colisiones. Si ya ha rebotado contra una pared, no vuelve a rebotar, se va
  (`parent.ReceiveActorBeginOverlap` OtherActor)
  (if (`KismetArrayLibrary.Array_Contains` (`Actor.Tags` OtherActor) "LateralHorizontal")
    (if (`self.HaRebotadoYa`)
      (`KismetSystemLibrary.Delay` 0.4)
      (`self.K2_DestroyActor`)
      (else
        (set `self.MovementVector` (* (`self.MovementVector`) -1.0))
        (set `self.HaRebotadoYa` true)))))

(event `self.ReceiveTick`
  (params (DeltaSeconds :type "Float (single-precision)"))
  ; Gira sobre sí mismo constantemente además de desplazarse
  (`parent.ReceiveTick` DeltaSeconds)
  (`self.K2_AddActorLocalRotation` (`KismetMathLibrary.MakeRotator` 0.0 0.0 (* DeltaSeconds (`self.RotationSpeed`)))))

(fn `Fire`
  (bind _firepoint4 (`self.FirePoint4`))
  (bind _firepoint (`self.FirePoint`))
  (bind _firepoint2 (`self.FirePoint2`))
  (bind _firepoint3 (`self.FirePoint3`))
  (`/Engine/EditorBlueprintResources/StandardMacros.IsValid` _firepoint
    (:`Is Valid`
      (`/Engine/EditorBlueprintResources/StandardMacros.IsValid` _firepoint2
        (:`Is Valid`
          (`/Engine/EditorBlueprintResources/StandardMacros.IsValid` _firepoint3
            (:`Is Valid`
              (`/Engine/EditorBlueprintResources/StandardMacros.IsValid` _firepoint4
                (:`Is Valid`
                  (`/Game/SpaceShooter/Players/BP_Pool.EnemyFire` (`self.M_Pool`) (`self.Ammo`) (`SceneComponent.K2_GetComponentToWorld` _firepoint) true (`SceneComponent.K2_GetComponentToWorld` _firepoint2) (`SceneComponent.K2_GetComponentToWorld` _firepoint3) (`SceneComponent.K2_GetComponentToWorld` _firepoint4)))))))))))

(fn `Move`
  (params (DeltaTime :type "Float (double-precision)"))
  (`parent.Move` DeltaTime))

(fn `UserConstructionScript`
  (`parent.UserConstructionScript`))