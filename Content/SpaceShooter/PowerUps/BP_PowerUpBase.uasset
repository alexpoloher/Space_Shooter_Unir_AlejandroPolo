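; Base power-up actor for the space shooter that drifts along its forward vector and is collected when the player character touches it.
; Tick moves it without sweep at a configurable speed, and BeginPlay caches the game mode.
; On overlap it passes its type to the character's AplicarPowerUp, then destroys itself after a brief delay.
; The pickup sound plays only for extra lives or when the character holds no power-up.
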(event `self.ReceiveBeginPlay`
  (bind _asbp_ss_game_mode (cast `/Game/BP_SS_GameMode` (`GameplayStatics.GetGameMode`)))
  (set `self.M_GameMode` _asbp_ss_game_mode))

(event `self.ReceiveTick`
  (params (DeltaSeconds :type "Float (single-precision)"))
  ; Gestionar movimiento
  (`self.K2_SetActorLocation` (+ (`self.K2_GetActorLocation`) (* (`self.GetActorForwardVector`) (* DeltaSeconds (`self.Speed`))))))

(event `self.ReceiveActorBeginOverlap`
  (params (OtherActor :type "Actor Object Reference"))
  ; Obtener PowerUp
  (bind _asbp_sspace_s_character (cast `/Game/SpaceShooter/Players/BP_SSpaceS_Character` OtherActor))
  (if (or (`KismetStringLibrary.EqualEqual_StrStr` (`self.TipoPowerUp`) "VidaExtra") (not (`/Game/SpaceShooter/Players/BP_SSpaceS_Character.TienePowerUp` _asbp_sspace_s_character)))
    (`GameplayStatics.PlaySound2D` (`self.Sonido`) 1.0 1.0 0.0 null null))
  (`/Game/SpaceShooter/Players/BP_SSpaceS_Character.AplicarPowerUp` _asbp_sspace_s_character (`self.TipoPowerUp`))
  (`KismetSystemLibrary.Delay` 0.1)
  (`self.K2_DestroyActor`))

(fn `UserConstructionScript`)