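; BP_SS_GameModeMenu appears to be the menu game mode, setting up a fixed view and mouse input.
; On BeginPlay it spawns an overhead orthographic CameraActor, makes it the first player controller's view target and shows the cursor.
; Gameplay events and the level-up and power-up selection functions are empty stubs, with only disconnected leftover nodes for health and weighted power-up spawn logic.
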(event `self.ReceiveBeginPlay`
  (bind _returnvalue (`GameplayStatics.GetPlayerController` 0))
  (bind _returnvalue_2 (`|SpawnActorFromClass` "/Script/Engine.CameraActor" (`KismetMathLibrary.MakeTransform` (0.0 0.0 1080.0) (struct :`Pitch` -90.0 :`Yaw` -180.0 :`Roll` 180.0)) "Undefined" "MultiplyWithRoot" null null))
  (`CameraComponent.SetProjectionMode` (`CameraActor.CameraComponent` _returnvalue_2) "Orthographic")
  (`CameraComponent.SetOrthoWidth` (`CameraActor.CameraComponent` _returnvalue_2) 2000.0)
  (`/Engine/EditorBlueprintResources/StandardMacros.IsValid` _returnvalue
    (:`Is Valid`
      (`PlayerController.SetViewTargetWithBlend` _returnvalue _returnvalue_2 0.0 "VTBlend_Linear" 0.0 false)
      (set `PlayerController.bShowMouseCursor` true (`GameplayStatics.GetPlayerController` 0)))))

(event `PlayerDead`)

(event `EnemyDestroyed`
  (params (PuntosExp :type Integer) (PosDestruccion :type "Vector Structure")))

(event `GetPowerUp`
  (params (TipoPowerUp :type String)))

(event `PerderPowerUp`)

(event `self.ReceiveTick`
  (params (DeltaSeconds :type "Float (single-precision)")))

(fn `GetPowerUpToSpawn`
  (params (RnadomInt :type Integer))
  (returns (Class :type "Actor Class Reference")))

(fn `SubirNivel`)

(fn `UserConstructionScript`)